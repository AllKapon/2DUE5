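; Player-controlled 2D flipbook character that runs along its forward axis and jumps.
; On BeginPlay it adds the movement Enhanced Input mapping context through its controller.
; Move input drives movement, switches between run and idle flipbooks, and rotates only the sprite to face the travel direction.
; An IsJumping flag blocks move input from the jump press until landing, which restores the looping idle flipbook.
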(event Input|EnhancedActionEvents|EnhancedInputActionIA_MoveForward
  (params (ActionValue :type Float%20%28double-precision%29) (ElapsedSeconds :type Float%20%28double-precision%29) (TriggeredSeconds :type Float%20%28double-precision%29) (InputAction :type Input%20Action%20Object%20Reference :default "/Game/Character/IA_MoveForward.IA_MoveForward"))
  (bind _sprite (Variables|Default|GetSprite))
  (:Triggered
    (if (not (Variables|Default|GetbIsJumping))
      (Pawn|Input|AddMovementInput (Transformation|GetActorForwardVector) ActionValue false)
      (Sprite|SetFlipbook _sprite "/Game/Character/Flipbooks/FB_Run.FB_Run")
      (if (> ActionValue 0.0)
        (Transformation|SetWorldRotation _sprite "0, 0, 0" false false)
        (else
          (Transformation|SetWorldRotation _sprite "0.000000,-180.000000,0.000000" false false)))))
  (:Canceled
    (Sprite|SetFlipbook _sprite "/Game/Character/Flipbooks/FB_Idle.FB_Idle" :!label _label))
  (:Completed
    (goto _label)))

(event Input|EnhancedActionEvents|EnhancedInputActionIA_Jump
  (params (ActionValue :type Boolean) (ElapsedSeconds :type Float%20%28double-precision%29) (TriggeredSeconds :type Float%20%28double-precision%29) (InputAction :type Input%20Action%20Object%20Reference :default "/Game/Character/IA_Jump.IA_Jump"))
  (:Triggered
    (Variables|Default|SetbIsJumping true)
    (Character|Jump)
    (Sprite|SetFlipbook (Variables|Default|GetSprite) "/Game/Character/Flipbooks/FB_Jump.FB_Jump")))

(event EventBeginPlay
  (bind _asmy_controler (Utilities|Casting|CastToMyControler (Pawn|GetController)))
  (Input|AddMappingContext (PlayerController|LocalPlayerSubsystems|GetEnhancedInputLocalPlayerSubsystem _asmy_controler) "/Game/Character/IMC_Movement.IMC_Movement" 0 "(bIgnoreAllPressedKeysUntilRelease=True,bForceImmediately=False,bNotifyUserSettings=False)"))

(event EventOnLanded
  (params (Hit :type Hit%20Result%20Structure%20%28by%20ref%29))
  (bind _sprite (Variables|Default|GetSprite))
  (Variables|Default|SetbIsJumping false)
  (Components|Timeline|SetLooping _sprite true)
  (Sprite|SetFlipbook _sprite "/Game/Character/Flipbooks/FB_Idle.FB_Idle"))

(fn ConstructionScript)